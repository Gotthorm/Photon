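; FlightPath_BP is an actor that displays a flight path as a translucent ribbon of spline meshes.
; Its construction script lays evenly spaced spline points along the actor's forward vector and creates segmented plane meshes along them.
; Update keeps the first point fixed, redistributes the others in a straight line to a target position, then reshapes and shows the existing meshes.
; Reset hides every segment.
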(event EventBeginPlay)

(event Collision|EventActorBeginOverlap
  (params (OtherActor :type Actor%20Object%20Reference)))

(event EventTick
  (params (DeltaSeconds :type Float%20%28single-precision%29)))

(fn ConstructionScript
  (LocalVariables|SetPosition%20Accumulator (Transformation|GetActorLocation))
  (bind _output_get (Variables|Default|SetFixed%20Spacing (/ (Variables|Default|GetLength) (Math|Conversions|ToFloat(Integer) (Variables|Default|GetSegmentCount)))))
  (for _index (range 0 (Variables|Default|GetSegmentCount))
    (bind _returnvalue (Utilities|Array|Add (LocalVariables|GetSpline%20Points) (+ (* (Transformation|GetActorForwardVector) _output_get) (LocalVariables|GetPosition%20Accumulator))))
    (bind _output_get_2 (LocalVariables|SetPosition%20Accumulator (+ (* (Transformation|GetActorForwardVector) _output_get) (LocalVariables|GetPosition%20Accumulator))))
    (Development|PrintText (Utilities|Text|FormatText "Added index: {index} position: {position} to array" (Utilities|Text|ToText(Integer) _returnvalue) (Utilities|Text|ToText(String) (Utilities|String|ToString(Vector) _output_get_2)))))
  (Spline|SetSplinePoints (Variables|Default|GetSpline) (LocalVariables|GetSpline%20Points) "World")
  (for _index_2 (range 0 (Variables|Default|GetSegmentCount))
    (bind _returnvalue_2 (AddComponent|AddSplineMeshComponent false))
    (Utilities|Array|Add (Variables|Default|GetSpline%20Mesh%20Array) _returnvalue_2)
    (Components|StaticMesh|SetStaticMesh _returnvalue_2 "/Game/Geometry/FlightPathPlane.FlightPathPlane")
    (Rendering|Material|SetMaterial _returnvalue_2 0 "/Game/Materials/TransparentUI.TransparentUI")
    (SplineMesh|SetStartandEnd _returnvalue_2 (Spline|GetLocationatDistanceAlongSpline (Variables|Default|GetSpline) (* _index_2 (Variables|Default|GetFixed%20Spacing)) "Local") (* (Spline|GetDirectionatDistanceAlongSpline (Variables|Default|GetSpline) (* _index_2 (Variables|Default|GetFixed%20Spacing)) "Local") (Variables|Default|GetFixed%20Spacing)) (Spline|GetLocationatDistanceAlongSpline (Variables|Default|GetSpline) (+ (* _index_2 (Variables|Default|GetFixed%20Spacing)) (Variables|Default|GetFixed%20Spacing)) "Local") (* (Spline|GetDirectionatDistanceAlongSpline (Variables|Default|GetSpline) (+ (* _index_2 (Variables|Default|GetFixed%20Spacing)) (Variables|Default|GetFixed%20Spacing)) "Local") (Variables|Default|GetFixed%20Spacing)) true :!class /Script/Engine.SplineMeshComponent)))

(fn Update
  (params (Target%20Position :type Vector))
  (bind _spline (Variables|Default|GetSpline))
  (LocalVariables|SetSpline%20Position (Spline|GetLocationatSplinePoint (Variables|Default|GetSpline) 0 "World"))
  (LocalVariables|SetSegment%20Vector (/ (- Target%20Position (LocalVariables|GetSpline%20Position)) (Variables|Default|GetSegmentCount)))
  (for _index (range 1 (Variables|Default|GetSegmentCount))
    (Spline|SetLocationatSplinePoint (Variables|Default|GetSpline) _index (+ (LocalVariables|GetSpline%20Position) (* (LocalVariables|GetSegment%20Vector) _index)) "World"))
  (Spline|UpdateSpline (Variables|Default|GetSpline))
  (for (_array_element _array_index) (Variables|Default|GetSpline%20Mesh%20Array)
    (Rendering|SetVisibility _array_element true false)
    (SplineMesh|SetStartandEnd _array_element (.Location (Spline|GetLocationandTangentatSplinePoint _spline _array_index "Local")) (.Tangent (Spline|GetLocationandTangentatSplinePoint _spline _array_index "Local")) (.Location (Spline|GetLocationandTangentatSplinePoint _spline (+ _array_index 1) "Local")) (.Tangent (Spline|GetLocationandTangentatSplinePoint _spline (+ _array_index 1) "Local")) true :!class /Script/Engine.SplineMeshComponent)
    (SplineMesh|UpdateMesh _array_element)))

(fn Reset
  ;[1 1 1] Set all of the spline mesh components to invisible
  (for _array_element (Variables|Default|GetSpline%20Mesh%20Array)
    (Rendering|SetVisibility _array_element false false)))